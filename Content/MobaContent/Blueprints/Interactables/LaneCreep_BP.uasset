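; LaneCreep_BP is a MOBA lane creep that follows a waypoint chain under AI control.
; On authority, its construction script sets its basic attack component and copies team and lane chain from the Bastion that instigated it.
; On BeginPlay it runs the LaneCreep_BT behavior tree and prints its team.
; Helper functions return the current waypoint and advance the index, stopping at the last one.
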(event `self.ReceiveBeginPlay`
  (bind _asaicontroller (cast `AIController` (`self.GetController`)))
  (`AIController.RunBehaviorTree` _asaicontroller "/Game/MobaContent/Blueprints/AI/LaneCreep_BT.LaneCreep_BT")
  (`KismetSystemLibrary.PrintString` (`KismetStringLibrary.Concat_StrStr` "I'm on team: " (`|GetEnumeratorNameAsString` (`self.Team`)))))

(fn `GetCurrentWaypoint`
  (returns (`Lane Point Location` :type "Vector Structure"))
  (bind _lane_point_location (`/Game/MobaContent/Blueprints/Misc/LaneWaypointChain.GetLanePoint` (`self.LaneWaypointChain`) (`self.LaneWaypointIndex`)))
  (return _lane_point_location))

(fn `IncWaypointIndex`
  (bind _lanewaypointindex (`self.LaneWaypointIndex`))
  (if (< _lanewaypointindex (- (`KismetArrayLibrary.Array_Length` (`/Game/MobaContent/Blueprints/Misc/LaneWaypointChain.LaneWaypoints` (`self.LaneWaypointChain`))) 1))
    (`/Engine/EditorBlueprintResources/StandardMacros.IncrementInt` _lanewaypointindex)))

(fn `UserConstructionScript`
  (`/Engine/EditorBlueprintResources/ActorMacros.Switch Has Authority`
    (:`Authority`
      (set `self.BasicInteract` (`self.BasicAttackComponent`))
      (bind _asbastion (cast `/Game/MobaContent/Blueprints/Interactables/Bastion` (`self.GetInstigator`)))
      (set `self.Team` (`Interactable.Team` _asbastion))
      (set `self.LaneWaypointChain` (`/Game/MobaContent/Blueprints/Interactables/Bastion.LaneWaypointChain` _asbastion)))))