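; Offensive MOBA structure, such as a defensive tower, that automatically fires its basic attack at enemies in range.
; RangeDetector overlaps take the first entrant from another team as target when none is valid, and clear it when that target leaves.
; Tick casts through the BasicAttackComponent while the target is valid.
; A DoOnce gate runs one closest-enemy search among overlapping Interactables when the target is lost, resetting while firing.
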(event OnComponentBeginOverlap(RangeDetector)
  (params (OtherActor :type Actor%20Object%20Reference) (OtherComp :type Primitive%20Component%20Object%20Reference) (OtherBodyIndex :type Integer) (bFromSweep :type Boolean) (SweepResult :type Hit%20Result%20Structure%20%28by%20ref%29))
  ;[1 1 1] Handle No Current Target - Target Enters Range
  (if (not (Utilities|IsValid (Variables|Default|GetCurrentFiringTarget)))
    (bind _asinteractable (Utilities|Casting|CastToInteractable OtherActor))
    (if (Utilities|Enum|NotEqual(Enum) (Variables|/Script/Moba.Interactable|GetTeam _asinteractable) (Variables|Default|GetTeam))
      (Variables|Default|SetCurrentFiringTarget OtherActor))))

(event OnComponentEndOverlap(RangeDetector)
  (params (OtherActor :type Actor%20Object%20Reference) (OtherComp :type Primitive%20Component%20Object%20Reference) (OtherBodyIndex :type Integer))
  ;[1 1 1] Handle Target Moved Out of Range
  (if (== OtherActor (Variables|Default|GetCurrentFiringTarget))
    (Variables|Default|SetCurrentFiringTarget 0)))

(event EventTick
  (params (DeltaSeconds :type Float%20%28single-precision%29))
  ;[1 1 1] Fire at enemy
  (if (Utilities|IsValid (Variables|Default|GetCurrentFiringTarget))
    (Class|Interactable|CastBasic (Variables|Default|GetCurrentFiringTarget)) ; This will use the basic attack component
    (goto _label Reset)
    (else
      ;[1 1 1] Attempt to acquire new target in range
      (Utilities|FlowControl|DoOnce false :!label _label
        (:Completed
          (bind _closest_in_range_enemy (CallFunction|FindClosestEnemyinRange))
          (Variables|Default|SetCurrentFiringTarget _closest_in_range_enemy))))))

(fn ConstructionScript
  (Variables|Default|SetBasicInteract (Variables|Default|GetBasicAttackComponent)))

(fn FindClosestEnemyinRange
  (for _array_element (Collision|GetOverlappingActors (Variables|Default|GetRangeDetector) "/Script/Moba.Interactable" :!class /Script/Engine.PrimitiveComponent)
    (bind _returnvalue (Class|Interactable|GetRelationship self _array_element))
    (switch Utilities|FlowControl|Switch|SwitchonERelationship _returnvalue
      (:Enemy
        (if (< (Transformation|GetDistanceTo _array_element) (LocalVariables|GetClosestDist))
          (LocalVariables|SetClosestDist (Transformation|GetDistanceTo _array_element))
          (bind _asinteractable (Utilities|Casting|CastToInteractable _array_element))
          (LocalVariables|SetClosestEnemy _asinteractable)))))
  (return (LocalVariables|GetClosestEnemy)))