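; Bastion is a MOBA structure that periodically spawns waves of lane creeps.
; On the server, Tick accumulates a wave timer that switches on spawn mode each time it reaches its maximum.
; While that mode is on, a second delay timer spaces out LaneCreep_BP spawns at the LaneWaypointChain transform, with the Bastion as Instigator.
; Spawn mode switches off and the counter resets once the wave's creep count is reached.
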(event `self.ReceiveBeginPlay`)

(event `self.ReceiveActorBeginOverlap`
  (params (OtherActor :type "Actor Object Reference")))

(event `self.ReceiveTick`
  (params (DeltaSeconds :type "Float (single-precision)"))
  (`parent.ReceiveTick` DeltaSeconds)
  (`/Engine/EditorBlueprintResources/ActorMacros.Switch Has Authority`
    (:`Authority`
      (`|ExecutionSequence`
        (:`then_0`
          ;[1 1 1] Handle Turning Spawn Mode on Every CreepSpawnTimerMax Seconds
          (bind _output_get (set `self.CreepSpawnTimer` (+ (`self.CreepSpawnTimer`) DeltaSeconds)))
          (if (>= _output_get (`self.CreepSpawnTimerMax`))
            (set `self.CreepSpawnTimer` 0.0)
            (set `self.CreepSpawnMode` true)))
        (:`then_1`
          ;[1 1 1] Handle Spawning Creeps When Spawn Mode is On
          (if (`self.CreepSpawnMode`)
            (set `self.CreepSpawnDelay` (+ (`self.CreepSpawnDelay`) DeltaSeconds))
            (if (>= (`self.CreepSpawnDelay`) (`self.CreepSpawnDelayMax`))
              (`|SpawnActorFromClass` "/Game/MobaContent/Blueprints/Interactables/LaneCreep_BP.LaneCreep_BP_C" (`self.GetTransform` (`self.LaneWaypointChain`)) "Undefined" "OverrideRootScale" null self)
              (bind _result (`/Engine/EditorBlueprintResources/StandardMacros.IncrementInt` (`self.NumCreepsSpawned`))
                (:`  `
                  (set `self.CreepSpawnDelay` 0.0)
                  (if (== _result (`self.NumCreepsToSpawn`))
                    (set `self.CreepSpawnMode` false)
                    (set `self.NumCreepsSpawned` 0)))))))))))

(fn `UserConstructionScript`
  (`parent.UserConstructionScript`))