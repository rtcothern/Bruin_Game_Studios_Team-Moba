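; Hero Blueprint in the MOBA interactables folder, holding what appears to be test logic for health and damage.
; Tick uses a one-second Delay as a throttle to repeatedly apply fixed damage to the hero itself and print RemainingHealth.
; An authority switch on Tick has empty branches.
; Disconnected nodes would add a Bolt ability component, test it and register it in Abilities, but never execute.
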(event `self.ReceiveBeginPlay`)

(event `self.ReceiveTick`
  (params (DeltaSeconds :type "Float (single-precision)"))
  (`/Engine/EditorBlueprintResources/ActorMacros.Switch Has Authority`
    (:`Authority`
      _)
    (:`Remote`
      _))
  (`KismetSystemLibrary.Delay` 1.0)
  (`GameplayStatics.ApplyDamage` self 20.0)
  (`KismetSystemLibrary.PrintString` (`KismetStringLibrary.Conv_IntToString` (`self.RemainingHealth`))))

(fn `UserConstructionScript`)