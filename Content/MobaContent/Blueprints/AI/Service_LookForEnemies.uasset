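; Behavior tree service that gives MOBA lane creeps an enemy target.
; On each AI tick it gets the Interactable actors overlapping the creep's AggroRangeDetector.
; The first one on a different team is written to the EnemyTarget blackboard key, with no distance ranking and no clearing when none is found.
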(event `self.ReceiveTickAI`
  (params (OwnerController :type "AIController Object Reference") (ControlledPawn :type "Pawn Object Reference") (DeltaSeconds :type "Float (single-precision)"))
  (bind _aslane_creep_bp (cast `/Game/MobaContent/Blueprints/Interactables/LaneCreep_BP` ControlledPawn))
  (for _array_element (`PrimitiveComponent.GetOverlappingActors` (`/Game/MobaContent/Blueprints/Interactables/LaneCreep_BP.AggroRangeDetector` _aslane_creep_bp) "/Script/Moba.Interactable")
    (bind _asinteractable (cast `Interactable` _array_element))
    (if (`|EnumInequality` (`Interactable.Team` _asinteractable) (`Interactable.Team` _aslane_creep_bp))
      (`BTFunctionLibrary.SetBlackboardValueAsObject` (`self.EnemyTarget`) _asinteractable)
      (break))))