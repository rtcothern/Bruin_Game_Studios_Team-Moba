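; Behavior tree task for a MOBA AI that chases an enemy and attacks it with a basic cast.
; On execute it reads the enemy from the blackboard, caches the pawn's basic interact range and issues a move without a target actor.
; Each tick it casts at the enemy when in range, otherwise moves toward it, using a DoOnce that resets when the move succeeds or fails.
; The task never calls finish.
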(event `self.ReceiveExecuteAI`
  (params (OwnerController :type "AIController Object Reference") (ControlledPawn :type "Pawn Object Reference"))
  (bind _asinteractable (cast `Interactable` (`BTFunctionLibrary.GetBlackboardValueAsObject` (`self.EnemyKey`))))
  (set `self.EnemyInteractable` _asinteractable)
  (bind _asinteractable_2 (cast `Interactable` ControlledPawn))
  (set `self.SelfInteractable` _asinteractable_2)
  (bind _output_get (set `self.AttackRange` (`KismetMathLibrary.Conv_IntToDouble` (`AbilityComponent.MaxRange` (`Interactable.BasicInteract` _asinteractable_2)))))
  (`|AIMoveTo` (`self.SelfInteractable`) (0.0 0.0 0.0) null _output_get))

(event `self.ReceiveTickAI`
  (params (OwnerController :type "AIController Object Reference") (ControlledPawn :type "Pawn Object Reference") (DeltaSeconds :type "Float (single-precision)"))
  (if (<= (`KismetMathLibrary.VSize` (- (`Actor.K2_GetActorLocation` ControlledPawn) (`Actor.K2_GetActorLocation` (`self.EnemyInteractable`)))) (`self.AttackRange`))
    (`Interactable.CastBasic` (`self.SelfInteractable`) (`self.EnemyInteractable`))
    (else
      (`/Engine/EditorBlueprintResources/StandardMacros.DoOnce` false :!label _label
        (:`Completed`
          (`|AIMoveTo` (`self.SelfInteractable`) (0.0 0.0 0.0) (`self.EnemyInteractable`) (`self.AttackRange`)
            (:`OnSuccess`
              (goto _label :!via `Reset`))
            (:`OnFail`
              (goto _label :!via `Reset`))))))))