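; Dash effect component that gives the affected character a temporary burst of walk speed.
; On apply, it saves the current max walk speed, multiplies it tenfold, sets a fixed duration and prints the saved speed on screen.
; Cleanup restores the saved speed on the affected character's Character Movement component.
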(event `OnApply`
  (bind _charactermovement (`Character.CharacterMovement` (`self.GetAffected`)))
  (bind _maxwalkspeed (`CharacterMovementComponent.MaxWalkSpeed` _charactermovement))
  (set `self.OldMaxSpeed` _maxwalkspeed)
  (set `CharacterMovementComponent.MaxWalkSpeed` (* _maxwalkspeed 10.0) _charactermovement)
  (set `self.Duration` 5.0)
  (`KismetSystemLibrary.PrintString` (`KismetStringLibrary.Conv_DoubleToString` (`self.OldMaxSpeed`)) true false (struct :`G` 0.097343 :`B` 0.61 :`A` 1.0)))

(event `self.Cleanup`
  (set `CharacterMovementComponent.MaxWalkSpeed` (`self.OldMaxSpeed`) (`Character.CharacterMovement` (`self.GetAffected`))))