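; Projectile actor for a bolt ability that damages the first enemy or neutral Interactable it hits.
; Sphere overlaps count only on the target's root component, then wait for a valid Source to resolve the relationship between the two.
; A qualifying hit applies fixed damage, prints the target's remaining health for debugging and destroys the bolt.
; Timed expiry with ability-end notification and a destination check are present but unwired.
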(event `self.SphereCollider.OnComponentBeginOverlap`
  (params (OtherActor :type "Actor Object Reference") (OtherComp :type "PrimitiveComponent Object Reference") (OtherBodyIndex :type Integer) (bFromSweep :type Boolean) (SweepResult :type "HitResult Structure (by ref)"))
  (bind _source (`self.Source`))
  (if (== (`self.K2_GetRootComponent` OtherActor) OtherComp)
    (bind _asinteractable (cast `Interactable` OtherActor))
    (`/Game/MobaContent/Blueprints/GameFramework/MobaMacroLibrary.WaitUntilValid` _source
      (:`exec out`
        (bind _returnvalue (`Interactable.GetRelationship` _source _asinteractable _source))
        (switch `ERelationship` _returnvalue
          (:`Enemy`
            _)
          (:`Neutral`
            _))
        (`GameplayStatics.ApplyDamage` OtherActor 100.0 null null "/Script/Engine.DamageType")
        (`KismetSystemLibrary.PrintString` (`KismetStringLibrary.Conv_IntToString` (`Interactable.RemainingHealth` _asinteractable)))
        (`self.K2_DestroyActor`)))))

(event `self.ReceiveTick`
  (params (DeltaSeconds :type "Float (single-precision)")))

(fn `UserConstructionScript`)