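; Bolt ability component for a MOBA, whose event graph holds only debug test scaffolding marked as currently broken.
; The Test event is empty, and a disconnected chain that never runs creates a Bolt_AOE evolution, adds it to Evos and makes it active.
; That chain then calls SkillUp on successive indices between delays, printing projectile pierce and size values to check the upgrades.
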(event `Test`)