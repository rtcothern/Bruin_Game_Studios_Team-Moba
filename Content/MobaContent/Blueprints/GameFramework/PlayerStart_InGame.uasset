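; In-game player start actor that hands out spawn points from a group of five child-actor starts.
; NextPlayerStart uses a counter to return the next child actor in round-robin order, wrapping back to the first after the fifth.
; It only rotates through the slots and does not check whether a start is occupied.
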(fn ConstructionScript)

(fn NextPlayerStart
  (switch int (Variables|Default|GetCounter)
    (:0
      (LocalVariables|SetPSToReturn (Variables|/Script/Engine.ChildActorComponent|GetChildActor (Variables|Default|GetStart%201)))
      (Math|Integer|IncrementInt (Variables|Default|GetCounter) :!label _label
        (:%20%20
          _)))
    (:1
      (LocalVariables|SetPSToReturn (Variables|/Script/Engine.ChildActorComponent|GetChildActor (Variables|Default|GetStart%202)))
      (goto _label))
    (:2
      (LocalVariables|SetPSToReturn (Variables|/Script/Engine.ChildActorComponent|GetChildActor (Variables|Default|GetStart%203)))
      (goto _label))
    (:3
      (LocalVariables|SetPSToReturn (Variables|/Script/Engine.ChildActorComponent|GetChildActor (Variables|Default|GetStart%204)))
      (goto _label))
    (:4
      (LocalVariables|SetPSToReturn (Variables|/Script/Engine.ChildActorComponent|GetChildActor (Variables|Default|GetStart%205)))
      (Variables|Default|SetCounter 0)))
  (return (LocalVariables|GetPSToReturn)))