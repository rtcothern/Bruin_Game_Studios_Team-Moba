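; GameState Blueprint for a MOBA match that tracks shared experience and levels for Team 1 and Team 2.
; GainExperience adds XP to the given team's total, then calls LevelUp, which raises that team's level once XP reaches a flat per-level threshold and subtracts the threshold.
; Each call grants at most one level, and crediting or leveling the Neutral team only prints a warning.
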(fn `GainExperience`
  (params (Team :type "ETeam Enum") (`Xp Gained` :type Integer))
  (switch `ETeam` Team
    (:`TeamA`
      (set `self.Team1Xp` (+ (`self.Team1Xp`) `Xp Gained`))
      (`self.LevelUp` Team :!label _label))
    (:`TeamB`
      (set `self.Team2Xp` (+ `Xp Gained` (`self.Team2Xp`)))
      (goto _label))
    (:`Neutral`
      (`KismetSystemLibrary.PrintText` "WARNING: attempted to credit Neutral team with experience" false))))

(fn `LevelUp`
  (params (Team :type "ETeam Enum"))
  (bind _xpperlevel (`self.XpPerLevel`))
  (bind _team2xp (`self.Team2Xp`))
  (bind _xpperlevel_2 (`self.XpPerLevel`))
  (bind _team1xp (`self.Team1Xp`))
  (switch `ETeam` Team
    (:`TeamA`
      (if (>= _team1xp _xpperlevel)
        (`/Engine/EditorBlueprintResources/StandardMacros.IncrementInt` (`self.Team1Level`)
          (:`  `
            (set `self.Team1Xp` (- _team1xp _xpperlevel))))))
    (:`TeamB`
      (if (>= _team2xp _xpperlevel_2)
        (`/Engine/EditorBlueprintResources/StandardMacros.IncrementInt` (`self.Team2Level`)
          (:`  `
            (set `self.Team2Xp` (- _team2xp _xpperlevel_2))))))
    (:`Neutral`
      (`KismetSystemLibrary.PrintString` "WARNING: attempting to level up neutral team" false))))

(fn `UserConstructionScript`)