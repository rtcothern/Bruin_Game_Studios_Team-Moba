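; In-game GameMode for a MOBA that handles team-based player start selection and delayed respawns.
; Respawn waits a per-team purgatory period, then on authority moves the player's existing character to the FindPlayerStart transform.
; ChoosePlayerStart caches one PlayerStart_InGame per team by tag on first call, then delegates to that actor's NextPlayerStart.
; PostLogin prints the joining player's name.
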(event `Respawn`
  (params (Controller :type "PlayerController Object Reference"))
  (bind _asmoba_player_controller (cast `MobaPlayerController` Controller))
  (switch `ETeam` (`MobaPlayerController.Team` _asmoba_player_controller)
    (:`TeamA`
      (`KismetSystemLibrary.Delay` (`self.Team1PurgatoryPeriod`)))
    (:`TeamB`
      (`KismetSystemLibrary.Delay` (`self.Team2PurgatoryPeriod`))))
  (`/Engine/EditorBlueprintResources/StandardMacros.IsValid` Controller
    (:`Is Valid`
      (`/Engine/EditorBlueprintResources/ActorMacros.Switch Has Authority`
        (:`Authority`
          (`self.K2_SetActorTransform` (`MobaPlayerController.PCharacter` _asmoba_player_controller) (`self.GetTransform` (`self.K2_FindPlayerStart` Controller)) false false))))))

(event `self.K2_PostLogin`
  (params (NewPlayer :type "PlayerController Object Reference"))
  (`KismetSystemLibrary.PrintString` (`KismetSystemLibrary.GetDisplayName` NewPlayer)))

(fn `ChoosePlayerStart`
  (params (Player :type "Controller Object Reference"))
  (returns (ReturnValue :type "Actor Object Reference"))
  (`|ExecutionSequence`
    (:`then_0`
      (`/Engine/EditorBlueprintResources/StandardMacros.DoOnce` false
        (:`Completed`
          ;[1 1 1] Acquire the Player Starts
          (bind _outactors (`GameplayStatics.GetAllActorsOfClass` "/Game/MobaContent/Blueprints/GameFramework/PlayerStart_InGame.PlayerStart_InGame_C"))
          (for _array_element _outactors
            (if (== "Team1" (`PlayerStart.PlayerStartTag` _array_element))
              (set `self.Team1Start` _array_element)
              (else
                (set `self.Team2Start` _array_element)))))))
    (:`then_1`
      (bind _aspcontroller_in_game (cast `/Game/MobaContent/Blueprints/GameFramework/Controllers/PController_InGame` Player))
      (switch `ETeam` (`MobaPlayerController.Team` _aspcontroller_in_game)
        (:`TeamA`
          (bind _player_start (`/Game/MobaContent/Blueprints/GameFramework/PlayerStart_InGame.Next Player Start` (`self.Team1Start`)))
          (return _player_start))
        (:`TeamB`
          (bind _player_start_2 (`/Game/MobaContent/Blueprints/GameFramework/PlayerStart_InGame.Next Player Start` (`self.Team2Start`)))
          (return _player_start_2))))))

(fn `UserConstructionScript`)